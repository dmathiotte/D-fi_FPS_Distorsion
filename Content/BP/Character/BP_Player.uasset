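; BP_Player is the player character, handling movement, camera look, jumping, running, crouching and door interaction.
; Movement follows control yaw, and Run switches walk speed while held.
; Jump fires only when there is no sideways or backward input.
; Interact runs a short debug-drawn visibility line trace from the camera and calls ActiveIt on a hit BP_Door.
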(event `InputAxis|Vertical`
  (params (AxisValue :type "Float (single-precision)"))
  (bind (_returnvalue_roll _returnvalue_pitch _returnvalue_yaw) (`KismetMathLibrary.BreakRotator` (`self.GetControlRotation`)))
  ;[1 1 1] Movement
  (`self.AddMovementInput` (`KismetMathLibrary.GetForwardVector` (`KismetMathLibrary.MakeRotator` 0.0 0.0 _returnvalue_yaw)) AxisValue))

(event `InputAxis|CamHorizontal`
  (params (AxisValue :type "Float (single-precision)"))
  ;[1 1 1] Cam
  (`self.AddControllerYawInput` AxisValue))

(event `InputAxis|CamVertical`
  (params (AxisValue :type "Float (single-precision)"))
  ;[1 1 1] Cam
  (`self.AddControllerPitchInput` AxisValue))

(event `InputAxis|Horizontal`
  (params (AxisValue :type "Float (single-precision)"))
  (bind (_returnvalue_roll _returnvalue_pitch _returnvalue_yaw) (`KismetMathLibrary.BreakRotator` (`self.GetControlRotation`)))
  ;[1 1 1] Movement
  (`self.AddMovementInput` (`KismetMathLibrary.GetRightVector` (`KismetMathLibrary.MakeRotator` 0.0 0.0 _returnvalue_yaw)) AxisValue))

(event `InputAction|Interact`
  (params (Key :type "Key Structure"))
  (bind _camera (`self.Camera`))
  (bind _returnvalue (`SceneComponent.K2_GetComponentLocation` _camera))
  ;[1 1 1] Interact
  (:`Pressed`
    (bind _outhit (`KismetSystemLibrary.LineTraceSingle` :`Start` _returnvalue :`End` (+ _returnvalue (* (`SceneComponent.GetForwardVector` _camera) 200.0)) :`TraceChannel` "TraceTypeQuery1" :`DrawDebugType` "ForDuration" :`DrawTime` 1.0))
    (bind _asbp_door (cast `/Game/BP/interactif/BP_Door` (`.HitActor` (`GameplayStatics.BreakHitResult` _outhit))))
    (`/Game/BP/interactif/BP_Door.ActiveIt` _asbp_door)))

(event `InputAction|Jump`
  (params (Key :type "Key Structure"))
  ;[1 1 1] Movement
  (:`Pressed`
    (if (and (>= (`self.GetInputAxisValue`) 0.0) (== (`self.GetInputAxisValue`) 0.0))
      (`self.Jump`)))
  (:`Released`
    (`self.StopJumping`)))

(event `InputAction|Run`
  (params (Key :type "Key Structure"))
  (bind _charactermovement (`self.CharacterMovement`))
  ;[1 1 1] Movement
  (:`Pressed`
    (set `CharacterMovementComponent.MaxWalkSpeed` 900.0 _charactermovement))
  (:`Released`
    (set `CharacterMovementComponent.MaxWalkSpeed` 600.0 _charactermovement)))

(event `InputAction|Crouch`
  (params (Key :type "Key Structure"))
  ;[1 1 1] Movement
  (:`Pressed`
    (`self.Crouch`))
  (:`Released`
    (`self.UnCrouch`)))

(fn `UserConstructionScript`)